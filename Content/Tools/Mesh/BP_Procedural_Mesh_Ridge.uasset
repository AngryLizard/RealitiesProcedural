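; Procedural mesh Blueprint tool that generates a ridge surface from Left and Right inputs.
; GenerateMesh passes both sides, a Curve and a material to GenerateRidge, using the Spread type with UV projection off.
; Filler spline and segment counts both scale from RidgeQuality, halving with each LOD level and rounding up.
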(fn ConstructionScript)

(fn GenerateMesh
  (params (Transform :type Transform%20%28by%20ref%29) (LOD :type Integer))
  (bind _returnvalue (Class|TGORMath|IntPow 0.5 LOD))
  (bind _ridgequality (Variables|Default|GetRidgeQuality))
  (bind _returnvalue_2 (* _ridgequality _returnvalue))
  (bind _returnvalue_3 (Math|Float|Ceil _returnvalue_2))
  (return (Class|TGORRidgeFillSplineLibrary|GenerateRidge (Variables|Default|GetLeft) (Variables|Default|GetRight) Transform (Utilities|Struct|MakeTGOR_RidgeSurfaceParams "0.000000,0.000000,1.000000" (Variables|Default|GetCurve) _returnvalue_3 _returnvalue_3) (Utilities|Struct|MakeTGOR_RidgeMaterialParams false 0.5 (Variables|Default|GetMaterial)) "Spread")))