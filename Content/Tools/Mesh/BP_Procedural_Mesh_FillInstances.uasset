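; Procedural mesh tool Blueprint that generates a Delaunay fill from Left and Right inputs, with holes, and covers it with mesh instances.
; GenerateMesh feeds Z-up surface, material, hole and tile extent, alignment and rotation settings into GenerateDelaunay.
; The resulting transforms populate the InstancedStaticMesh component, and the generated meshes are returned to the caller.
; The LOD input is unused, and the event graph and construction script are empty.
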(event EventBeginPlay)

(event Collision|EventActorBeginOverlap
  (params (OtherActor :type Actor%20Object%20Reference)))

(event EventTick
  (params (DeltaSeconds :type Float%20%28single-precision%29)))

(fn ConstructionScript)

(fn GenerateMesh
  (params (Transform :type Transform%20%28by%20ref%29) (LOD :type Integer))
  (bind _tgor_delaunaysurfaceparams (Utilities|Struct|MakeTGOR_DelaunaySurfaceParams "0.000000,0.000000,1.000000" 0 5e+01))
  (bind _left (Variables|Default|GetLeft))
  (bind _right (Variables|Default|GetRight))
  (bind _holeradius (Variables|Default|GetHoleRadius))
  (bind _rotations (Variables|Default|GetRotations))
  (bind _alignments (Variables|Default|GetAlignments))
  (bind _tileextend (Variables|Default|GetTileExtend))
  (bind _material (Variables|Default|GetMaterial))
  (bind _hs (Variables|Default|GetHs))
  (bind _tgor_delaunayinstanceparams (Utilities|Struct|MakeTGOR_DelaunayInstanceParams _tileextend _alignments _rotations))
  (bind _tgor_delaunayholeparams (Utilities|Struct|MakeTGOR_DelaunayHoleParams _holeradius _hs))
  (bind _tgor_delaunaymaterialparams (Utilities|Struct|MakeTGOR_DelaunayMaterialParams false _material))
  (bind (_meshes _transforms) (Class|TGORDelaunayFillSplineLibrary|GenerateDelaunay _left _right Transform _tgor_delaunaysurfaceparams _tgor_delaunaymaterialparams _tgor_delaunayinstanceparams _tgor_delaunayholeparams))
  (Class|TGORProceduralLibrary|PopulateInstancedMesh (Variables|Default|GetInstancedStaticMesh) _transforms)
  (return _meshes))