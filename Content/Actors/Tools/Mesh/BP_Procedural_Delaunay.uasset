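; Procedural mesh tool Blueprint that builds a Delaunay-triangulated surface from Left and Right inputs, curves and an up vector, with support for holes.
; GenerateMesh passes surface, material, instance and hole parameters to GenerateDelaunay and returns the resulting meshes.
; The generated transforms also populate an instanced static mesh component.
; Filler max size doubles with each LOD level, so triangulation coarsens at higher LODs.
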(fn ConstructionScript)

(fn GenerateMesh
  (params (Transform :type Transform%20%28by%20ref%29) (LOD :type Integer))
  (bind _returnvalue (Class|TGORMath|IntPow 2.0 LOD))
  (bind _left (Variables|Default|GetLeft))
  (bind _filler_max_size (Variables|Default|GetFiller%20Max%20Size))
  (bind _delaunay (Variables|Default|GetDelaunay))
  (bind _instance_extend (Variables|Default|GetInstance%20Extend))
  (bind _rotate_along_principal (Variables|Default|GetRotate%20Along%20Principal))
  (bind _right (Variables|Default|GetRight))
  (bind _material (Variables|Default|GetMaterial))
  (bind _holes (Variables|Default|GetHoles))
  (bind _upvector (Variables|Default|GetUpVector))
  (bind _curves (Variables|Default|GetCurves))
  (bind _returnvalue_2 (* _filler_max_size _returnvalue))
  (bind _tgor_delaunaymaterialparams (Utilities|Struct|MakeTGOR_DelaunayMaterialParams false _material))
  (bind _tgor_delaunayholeparams (Utilities|Struct|MakeTGOR_DelaunayHoleParams 1e+02 _holes))
  (bind _tgor_delaunayinstanceparams (Utilities|Struct|MakeTGOR_DelaunayInstanceParams _instance_extend 0 0 true _rotate_along_principal))
  (bind _tgor_delaunaysurfaceparams (Utilities|Struct|MakeTGOR_DelaunaySurfaceParams _upvector _curves _returnvalue_2 1e+02 _delaunay))
  (bind (_meshes _transforms) (Class|TGORDelaunayFillSplineLibrary|GenerateDelaunay _left _right Transform _tgor_delaunaysurfaceparams _tgor_delaunaymaterialparams _tgor_delaunayinstanceparams _tgor_delaunayholeparams))
  (Class|TGORProceduralLibrary|PopulateInstancedMesh (Variables|Default|GetInstancedStaticMesh) _transforms)
  (return _meshes))