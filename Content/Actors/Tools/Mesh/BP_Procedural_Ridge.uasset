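; BP_Procedural_Ridge is a procedural mesh tool that generates a ridge from its Left and Right inputs.
; GenerateMesh passes the transform and ridge type to GenerateRidge, along with surface parameters (up vector, curve, filler splines and segments) and material parameters.
; Filler segments are divided by LOD + 1, so higher LOD indices get coarser geometry.
; UV projection is disabled, with the unwrap lane setting passed instead.
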(fn ConstructionScript)

(fn GenerateMesh
  (params (Transform :type Transform%20%28by%20ref%29) (LOD :type Integer))
  (return (Class|TGORRidgeFillSplineLibrary|GenerateRidge (Variables|Default|GetLeft) (Variables|Default|GetRight) Transform (Utilities|Struct|MakeTGOR_RidgeSurfaceParams (Variables|Default|GetUpVector) (Variables|Default|GetCurve) (Variables|Default|GetFiller%20Splines) (/ (Variables|Default|GetFiller%20Segments) (+ LOD 1))) (Utilities|Struct|MakeTGOR_RidgeMaterialParams false (Variables|Default|GetUnwrap%20Lane) (Variables|Default|GetMaterial)) (Variables|Default|GetType))))