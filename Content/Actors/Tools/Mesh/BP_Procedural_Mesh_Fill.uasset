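; Procedural mesh tool actor that generates a filled, thick surface from a spline.
; GenerateMesh passes the spline, transform, up vector and thickness to GenerateFill, with one material for top and bottom and another for the rim.
; The curve threshold doubles with each LOD level, presumably coarsening the spline sampling for lower-detail meshes.
; The construction script is empty.
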(fn ConstructionScript)

(fn GenerateMesh
  (params (Transform :type Transform%20%28by%20ref%29) (LOD :type Integer))
  (bind _material (Variables|Default|GetMaterial))
  (return (Class|TGORFillDelaunayLibrary|GenerateFill (Variables|Default|GetSpline) Transform (Utilities|Struct|MakeTGOR_FillSurfaceParams (Variables|Default|GetUpVector) (* (Variables|Default|GetFillerThreshold) (Class|TGORMath|IntPow 2.0 LOD)) true (Variables|Default|GetThickness)) (Utilities|Struct|MakeTGOR_FillMaterialParams _material (Variables|Default|GetRim) _material))))